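; BP_Canon is a cannon actor that repeatedly fires projectiles on its own from BeginPlay.
; After a FireRate delay, it spawns a BP_Projectile at the spawn point's transform, scaled by ProjectileScale, ignoring collision.
; The CanonMove timeline then animates the cannon mesh along its local Y axis.
; The timeline's Canon Fired event track loops execution back to the delay, driving the next shot.
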(event EventBeginPlay
  (Utilities|FlowControl|Delay (Variables|CannonFireProperties|GetFireRate) :!label _label)
  (CallFunction|SpawnProjectile)
  (bind _translatecanon (Timeline|CanonMove PlayFromStart)
    (:Update
      (Transformation|SetRelativeLocation (Variables|Default|GetCanon) (Math|Vector|MakeVector 0.0 _translatecanon 0.0) false false))
    (:CanonFired
      (goto _label))))

(fn ConstructionScript)

(fn SpawnProjectile
  (bind _projectilspawnpoint (Variables|Default|GetProjectilSpawnPoint))
  (bind _returnvalue (Transformation|GetWorldTransform _projectilspawnpoint))
  (Game|SpawnActorfromClass "/Game/Blueprints/Actors/Projectiles/BP_Projectile.BP_Projectile_C" (Math|Transform|MakeTransform (.location _returnvalue) (.rotation _returnvalue) (Math|Conversions|ToVector(Float) (Variables|CannonFireProperties|GetProjectileScale))) "AlwaysSpawn" 0 0))