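; Collectable crystal actor that flies into the player pawn, shrinking and dimming, when the player overlaps it.
; The overlap stores its starting location, scale and light intensity, then plays the Collection timeline unless already at the player, where it stops it instead.
; Timeline curves lerp location toward the player's live position and fade scale and point light to zero.
; The actor destroys itself when the timeline finishes.
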(event Collision|EventActorBeginOverlap
  (params (OtherActor :type Actor%20Object%20Reference))
  (CallFunction|SetStartVariables)
  (Utilities|CheckColiderIsPlayer OtherActor
    (:then
      (Utilities|CheckLocationatPlayer
        (:then
          (bind (_direction _smoothmovealpha _smoothsizealpha _smoothalphalight) (Timeline|Collection Stop)
            (:Update
              (CallFunction|MovetoPlayerandShrink _smoothmovealpha)
              (CallFunction|ChangeCrystalSize _smoothsizealpha)
              (CallFunction|ChangeLightIntensity _smoothalphalight))
            (:Finished
              (Actor|DestroyActor))))
        (:else
          (Timeline|Collection Play))))))

(fn ConstructionScript)

(fn MovetoPlayerandShrink
  (params (SmoothMoveAlpha :type Float%20%28single-precision%29))
  (Transformation|SetActorLocation (Math|Vector|Lerp(Vector) (Variables|Default|GetStartLerpLocation) (Transformation|GetActorLocation (Game|Player|GetPlayerPawn 0)) SmoothMoveAlpha) false false))

(fn SetStartVariables
  (Variables|Default|SetStartLerpLocation (Transformation|GetActorLocation))
  (Variables|Default|SetStartLerpSize (Transformation|GetActorScale3D))
  (Variables|Default|SetStartLightIntensity (Variables|/Script/Engine.LightComponentBase|GetIntensity (Variables|Default|GetPointLight))))

(fn CheckLocationtoPlayer
  (return (Math|Vector|Equal(Vector) (Transformation|GetActorLocation) (Transformation|GetActorLocation (Game|Player|GetPlayerPawn 0)) 1e+01)))

(fn ChangeCrystalSize
  (params (Alpha :type Float%20%28single-precision%29))
  (Transformation|SetActorScale3D (Math|Vector|Lerp(Vector) (Variables|Default|GetStartLerpSize) "0, 0, 0" Alpha)))

(fn ChangeLightIntensity
  (params (SmoothAlphaLight :type Float%20%28single-precision%29))
  (Rendering|Components|Light|SetIntensity (Variables|Default|GetPointLight) (Math|Float|Lerp (Variables|Default|GetStartLightIntensity) 0.0 SmoothAlphaLight)))