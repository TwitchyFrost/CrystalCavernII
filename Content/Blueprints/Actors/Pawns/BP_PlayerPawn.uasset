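; Player pawn that moves by applying torque to its physics-driven static mesh and restarts the level when damaged.
; Forward/Back and Left/Right axis inputs add scaled torque around the world Y and X axes as an acceleration change, ignoring mass.
; The camera fades in on BeginPlay.
; The first damage event of any amount, gated by DoOnce, fades the camera out, waits for the fade, then reloads the current level by name.
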(event EventBeginPlay
  (CameraFades|StartCameraFade :self (Game|GetPlayerCameraManager 0) :FromAlpha 1.0 :Duration 2.0))

(event Game|Damage|EventAnyDamage
  (params (Damage :type Float%20%28single-precision%29) (DamageType :type Damage%20Type%20Object%20Reference) (InstigatedBy :type Controller%20Object%20Reference) (DamageCauser :type Actor%20Object%20Reference))
  (Utilities|FlowControl|DoOnce false
    (:Completed
      (CameraFades|StartCameraFade :self (Game|GetPlayerCameraManager 0) :ToAlpha 1.0 :Duration (Variables|Default|GetFadeTime) :bHoldWhenFinished true)
      (Utilities|FlowControl|Delay (Variables|Default|GetFadeTime))
      (bind _returnvalue (Game|GetCurrentLevelName true))
      (Game|OpenLevel(byName) (Utilities|String|StringToName _returnvalue)))))

(event Input|AxisEvents|InputAxisForward/Back
  (params (AxisValue :type Float%20%28single-precision%29))
  (Class|PrimitiveComponent|AddTorqueinRadians (Variables|Default|GetStaticMesh) (Math|Vector|MakeVector 0.0 (* AxisValue (Variables|Default|GetTorqueScale)) 0.0) "None" true))

(event Input|AxisEvents|InputAxisLeft/Right
  (params (AxisValue :type Float%20%28single-precision%29))
  (Class|PrimitiveComponent|AddTorqueinRadians (Variables|Default|GetStaticMesh) (Math|Vector|MakeVector (* AxisValue (Variables|Default|GetTorqueScale)) 0.0 0.0) "None" true))

(fn ConstructionScript)